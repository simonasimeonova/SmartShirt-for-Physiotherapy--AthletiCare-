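; BP_ChartManager records daily score entries for a chart in the SG_ChartData save game.
; StoreTodayScore pairs a date string built from the current time with a random placeholder average, rather than a measured score.
; It loads or creates the save slot, appends the entry, saves, and fires OnDoneSaving.
; Init is empty, and the logic trimming old entries is disconnected, so history is never capped.
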(event `self.ReceiveInit`)

(fn `StoreTodayScore`
  (locals (TodayString :type String))
  (bind _returnvalue (`KismetStringLibrary.ParseIntoArray` (`KismetTextLibrary.Conv_TextToString` (`KismetTextLibrary.AsTimeZoneDateTime_DateTime` (`KismetMathLibrary.Now`)))))
  (set `self.Average` (`KismetMathLibrary.RandomIntegerInRange` 60 99))
  (set `local.TodayString` (`KismetTextLibrary.Conv_TextToString` (`|FormatText` "{A} {B}" (`|GetArrayItem` _returnvalue) (`|GetArrayItem` _returnvalue 1))))
  (bind _returnvalue_2 (`GameplayStatics.DoesSaveGameExist` "ChartDataSlot"))
  (if _returnvalue_2
    (bind _returnvalue_3 (`GameplayStatics.LoadGameFromSlot` "ChartDataSlot"))
    (bind _assg_chart_data (cast `/Game/SportRehab/Blueprints/SG_ChartData` _returnvalue_3))
    (set `self.SaveRef` _assg_chart_data)
    (else
      (bind _returnvalue_4 (`GameplayStatics.CreateSaveGameObject` "/Game/SportRehab/Blueprints/SG_ChartData.SG_ChartData_C"))
      (set `self.SaveRef` _returnvalue_4)
      (`KismetSystemLibrary.PrintString` "created")))
  (`KismetArrayLibrary.Array_Add` (`/Game/SportRehab/Blueprints/SG_ChartData.DailyEntries` (`self.SaveRef`)) (make `/Game/SportRehab/Blueprints/ST_DailyScore` (`local.TodayString`) (`self.Average`)))
  (bind _returnvalue_5 (`GameplayStatics.SaveGameToSlot` (`self.SaveRef`) "ChartDataSlot"))
  (`self.OnDoneSaving` _returnvalue_5))