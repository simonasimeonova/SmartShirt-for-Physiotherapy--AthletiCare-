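; Actor that drives a PoseableMesh's arms from sensor quaternions received over local OSC and counts exercise reps.
; After a delayed calibration against ReferenceMesh bones, Tick applies offset, mirrored rotations to both upper and lower arms; torso driving is unused.
; Collision components follow both hands, but only right-hand overlaps with tagged targets count reps or warn when too slow.
; Dispatchers report calibration, rep progress, sets, resets and warnings.
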(event `OnQuat0Received`
  (params (AddressPattern :type "OSCAddress Structure (by ref)") (Message :type "OSCMessage Structure (by ref)") (IPAddress :type String) (Port :type Integer))
  (bind _values (`OSCManager.GetAllFloats` Message))
  (set `self.Quat_0` (`KismetMathLibrary.MakeQuat` (`|GetArrayItem` _values) (`|GetArrayItem` _values 1) (`|GetArrayItem` _values 2) (`|GetArrayItem` _values 3))))

(event `OnQuat1Received`
  (params (AddressPattern :type "OSCAddress Structure (by ref)") (Message :type "OSCMessage Structure (by ref)") (IPAddress :type String) (Port :type Integer))
  (bind _values (`OSCManager.GetAllFloats` Message))
  (set `self.Quat_1` (`KismetMathLibrary.MakeQuat` (`|GetArrayItem` _values) (`|GetArrayItem` _values 1) (`|GetArrayItem` _values 2) (`|GetArrayItem` _values 3))))

(event `self.ReceiveBeginPlay`
  (bind _returnvalue (`OSCManager.CreateOSCServer` "127.0.0.1" 5001 false true "" null))
  (set `self.OSCServer` _returnvalue)
  (`KismetSystemLibrary.LogString` "Set OSCServer.")
  (`|ExecutionSequence`
    (:`then_0`
      (bind _returnvalue_2 (`OSCManager.ConvertStringToOSCAddress` "/quat/0"))
      (`OSCServer.BindEventToOnOSCAddressPatternMatchesPath` (`self.OSCServer`) _returnvalue_2 (delegate `OnQuat0Received`)))
    (:`then_1`
      (bind _returnvalue_3 (`OSCManager.ConvertStringToOSCAddress` "/quat/1"))
      (`OSCServer.BindEventToOnOSCAddressPatternMatchesPath` (`self.OSCServer`) _returnvalue_3 (delegate `OnQuat1Received`)))
    (:`then_2`
      (bind _returnvalue_4 (`OSCManager.ConvertStringToOSCAddress` "/quat/2"))
      (`OSCServer.BindEventToOnOSCAddressPatternMatchesPath` (`self.OSCServer`) _returnvalue_4 (delegate `OnQuat2Received`)))
    (:`then_3`
      (bind _returnvalue_5 (`OSCManager.ConvertStringToOSCAddress` "/quat/3"))
      (`OSCServer.BindEventToOnOSCAddressPatternMatchesPath` (`self.OSCServer`) _returnvalue_5 (delegate `OnQuat3Received`)))
    (:`then_4`
      (bind _returnvalue_6 (`OSCManager.ConvertStringToOSCAddress` "/quat/4"))
      (`OSCServer.BindEventToOnOSCAddressPatternMatchesPath` (`self.OSCServer`) _returnvalue_6 (delegate `OnQuat4Received`))))
  (`KismetSystemLibrary.Delay` 0.1)
  (`self.OnInitialCalibration`)
  (`KismetSystemLibrary.Delay` 3.0)
  (`self.CalibrateSensors`)
  (`KismetSystemLibrary.Delay` 3.0)
  (`KismetSystemLibrary.PrintString` "Finished calibration" false true (struct :`G` 0.66 :`B` 1.0 :`A` 1.0) 1e+19)
  (`self.OnEndInitialCalibration`))

(event `OnQuat2Received`
  (params (AddressPattern :type "OSCAddress Structure (by ref)") (Message :type "OSCMessage Structure (by ref)") (IPAddress :type String) (Port :type Integer))
  (bind _values (`OSCManager.GetAllFloats` Message))
  (set `self.Quat_2` (`KismetMathLibrary.MakeQuat` (`|GetArrayItem` _values) (`|GetArrayItem` _values 1) (`|GetArrayItem` _values 2) (`|GetArrayItem` _values 3))))

(event `OnQuat3Received`
  (params (AddressPattern :type "OSCAddress Structure (by ref)") (Message :type "OSCMessage Structure (by ref)") (IPAddress :type String) (Port :type Integer))
  (bind _values (`OSCManager.GetAllFloats` Message))
  (set `self.Quat_3` (`KismetMathLibrary.MakeQuat` (`|GetArrayItem` _values) (`|GetArrayItem` _values 1) (`|GetArrayItem` _values 2) (`|GetArrayItem` _values 3))))

(event `OnQuat4Received`
  (params (AddressPattern :type "OSCAddress Structure (by ref)") (Message :type "OSCMessage Structure (by ref)") (IPAddress :type String) (Port :type Integer))
  (bind _values (`OSCManager.GetAllFloats` Message))
  (set `self.Quat_4` (`KismetMathLibrary.MakeQuat` (`|GetArrayItem` _values) (`|GetArrayItem` _values 1) (`|GetArrayItem` _values 2) (`|GetArrayItem` _values 3))))

(event `self.ReceiveTick`
  (params (DeltaSeconds :type "Float (single-precision)"))
  (if (`self.isCalibrated`)
    (bind _outquat (`self.MirrorQuatLR` (`self.Quat_0`)))
    (`PoseableMeshComponent.SetBoneRotationByName` (`self.PoseableMesh`) "upperarm_r" (`KismetMathLibrary.Quat_Rotator` (* (`self.Quat_0_Offset`) _outquat)) "ComponentSpace")
    (bind _outquat_2 (`self.MirrorQuatLR` (`self.Quat_1`)))
    (bind _outquat_3 (`self.MirrorQuatFB` (* (`self.Quat_1_Offset`) _outquat_2)))
    (`PoseableMeshComponent.SetBoneRotationByName` (`self.PoseableMesh`) "upperarm_l" (`KismetMathLibrary.Quat_Rotator` _outquat_3) "ComponentSpace")
    (bind _outquat_4 (`self.MirrorQuatLR` (`self.Quat_2`)))
    (`PoseableMeshComponent.SetBoneRotationByName` (`self.PoseableMesh`) "lowerarm_r" (`KismetMathLibrary.Quat_Rotator` (* (`self.Quat_2_Offset`) _outquat_4)) "ComponentSpace")
    (bind _outquat_5 (`self.MirrorQuatLR` (`self.Quat_3`)))
    (bind _outquat_6 (`self.MirrorQuatFB` (* (`self.Quat_3_Offset`) _outquat_5)))
    (`PoseableMeshComponent.SetBoneRotationByName` (`self.PoseableMesh`) "lowerarm_l" (`KismetMathLibrary.Quat_Rotator` _outquat_6) "ComponentSpace")
    (bind _returnvalue (`PoseableMeshComponent.GetBoneTransformByName` (`self.PoseableMesh`) "hand_l" "WorldSpace"))
    (`SceneComponent.K2_SetWorldTransform` (`self.LeftHandCollision`) (`KismetMathLibrary.MakeTransform` (.location _returnvalue) (.rotation _returnvalue) (0.3 0.3 0.3)) false false)
    (bind _returnvalue_2 (`PoseableMeshComponent.GetBoneTransformByName` (`self.PoseableMesh`) "hand_r" "WorldSpace"))
    (`SceneComponent.K2_SetWorldTransform` (`self.RightHandCollision`) (`KismetMathLibrary.MakeTransform` (.location _returnvalue_2) (.rotation _returnvalue_2) (0.3 0.3 0.3)) false false)))

(event `HandleRep`
  (`/Engine/EditorBlueprintResources/StandardMacros.IncrementFloat` (`self.Current Rep`)
    (:`  `
      (switch `int` (`self.CurrentExercise`)
        (:`0`
          (set `self.RepsPerSet` 5.0))
        (:`1`
          (set `self.RepsPerSet` 5.0))
        (:`2`
          (set `self.RepsPerSet` 3.0)))
      (`self.OnRepProgress` (/ (`self.Current Rep`) (`self.RepsPerSet`)) (`KismetMathLibrary.FTrunc` (`self.Current Rep`)))
      (if (== (`self.Current Rep`) (`self.RepsPerSet`))
        (`self.HandleSetCompleted`)))))

(event `HandleSetCompleted`
  (`/Engine/EditorBlueprintResources/StandardMacros.IncrementInt` (`self.CurrentSet`)
    (:`  `
      (set `self.Current Rep` 0.0)
      (`self.OnSetCompleted` (`self.CurrentSet`) (`self.CurrentExercise`))
      (if (== (`self.CurrentSet`) 2)
        (`self.ResetExercise`)))))

(event `ResetExercise`
  (set `self.CurrentSet` 0)
  (set `self.Current Rep` 0.0)
  (`self.OnExerciseReset`))

(event `self.LeftHandCollision.OnComponentBeginOverlap`
  (params (OverlappedComponent :type "PrimitiveComponent Object Reference") (OtherActor :type "Actor Object Reference") (OtherComp :type "PrimitiveComponent Object Reference") (OtherBodyIndex :type Integer) (bFromSweep :type Boolean) (SweepResult :type "HitResult Structure (by ref)")))

(event `self.RightHandCollision.OnComponentBeginOverlap`
  (params (OverlappedComponent :type "PrimitiveComponent Object Reference") (OtherActor :type "Actor Object Reference") (OtherComp :type "PrimitiveComponent Object Reference") (OtherBodyIndex :type Integer) (bFromSweep :type Boolean) (SweepResult :type "HitResult Structure (by ref)"))
  (if (and (`self.ActorHasTag` OtherActor "overhead") (== (`self.CurrentExercise`) 0))
    (if (and (> (- (`KismetSystemLibrary.GetGameTimeInSeconds`) (`self.LastOverheadOverlap`)) 4.0) (> (`self.Current Rep`) 1.0))
      (`GameplayStatics.PlaySound2D` "/Game/SportRehab/Characters/Animations/Sounds/dont_give_up.dont_give_up" 1.0 1.0 0.0 null null)
      (`self.OnWarningRaised`)
      (else
        (`self.HandleRep`)))
    (set `self.LastOverheadOverlap` (`KismetSystemLibrary.GetGameTimeInSeconds`))
    (elif (and (`self.ActorHasTag` OtherActor "shoulder") (== (`self.CurrentExercise`) 1))
      (if (and (> (- (`KismetSystemLibrary.GetGameTimeInSeconds`) (`self.LastLateralOverlap`)) 4.0) (> (`self.Current Rep`) 1.0))
        (`GameplayStatics.PlaySound2D` "/Game/SportRehab/Characters/Animations/Sounds/dont_give_up.dont_give_up" 1.0 1.0 0.0 null null)
        (`self.OnWarningRaised`)
        (else
          (`self.HandleRep`)))
      (set `self.LastLateralOverlap` (`KismetSystemLibrary.GetGameTimeInSeconds`))
      (elif (and (`self.ActorHasTag` OtherActor "overhead") (== (`self.CurrentExercise`) 2))
        (if (and (> (- (`KismetSystemLibrary.GetGameTimeInSeconds`) (`self.LastYTWOverlap`)) 4.0) (> (`self.Current Rep`) 1.0))
          (`GameplayStatics.PlaySound2D` "/Game/SportRehab/Characters/Animations/Sounds/dont_give_up.dont_give_up" 1.0 1.0 0.0 null null)
          (`self.OnWarningRaised`)
          (else
            (`self.HandleRep`)))
        (set `self.LastYTWOverlap` (`KismetSystemLibrary.GetGameTimeInSeconds`))))))

(event `CalibrateSensors`
  (bind _outquat (`self.MirrorQuatLR` (`self.Quat_0`)))
  (bind _offset_0 (`self.ComputeOffset0` _outquat))
  (set `self.Quat_0_Offset` _offset_0)
  (bind _outquat_2 (`self.MirrorQuatLR` (`self.Quat_1`)))
  (bind _offset_1 (`self.ComputeOffset1` _outquat_2))
  (set `self.Quat_1_Offset` _offset_1)
  (bind _outquat_3 (`self.MirrorQuatLR` (`self.Quat_2`)))
  (bind _offset_2 (`self.ComputeOffset2` _outquat_3))
  (set `self.Quat_2_Offset` _offset_2)
  (bind _outquat_4 (`self.MirrorQuatLR` (`self.Quat_3`)))
  (bind _offset_3 (`self.ComputeOffset3` _outquat_4))
  (set `self.Quat_3_Offset` _offset_3)
  (bind _outquat_5 (`self.MirrorQuatLR` (`self.Quat_4`)))
  (bind _offset_4 (`self.ComputeOffset4` _outquat_5))
  (set `self.Quat_4_Offset` _offset_4)
  (set `self.isCalibrated` true))

(fn `ComputeOffset0`
  (params (Quat_0 :type "Quat Structure"))
  (returns (Offset_0 :type "Quat Structure"))
  (return (* (`KismetMathLibrary.Conv_RotatorToQuaternion` (.rotation (`SkinnedMeshComponent.GetBoneTransform` (`self.ReferenceMesh`) "upperarm_r" "RTS_Component"))) (`KismetMathLibrary.Quat_Inversed` Quat_0))))

(fn `ComputeOffset1`
  (params (Quat_1 :type "Quat Structure"))
  (returns (Offset_1 :type "Quat Structure"))
  (return (* (`KismetMathLibrary.Conv_RotatorToQuaternion` (.rotation (`SkinnedMeshComponent.GetBoneTransform` (`self.ReferenceMesh`) "upperarm_l" "RTS_Component"))) (`KismetMathLibrary.Quat_Inversed` Quat_1))))

(fn `ComputeOffset2`
  (params (Quat_2 :type "Quat Structure"))
  (returns (Offset_2 :type "Quat Structure"))
  (return (* (`KismetMathLibrary.Conv_RotatorToQuaternion` (.rotation (`SkinnedMeshComponent.GetBoneTransform` (`self.ReferenceMesh`) "lowerarm_r" "RTS_Component"))) (`KismetMathLibrary.Quat_Inversed` Quat_2))))

(fn `ComputeOffset3`
  (params (Quat_3 :type "Quat Structure"))
  (returns (Offset_3 :type "Quat Structure"))
  (return (* (`KismetMathLibrary.Conv_RotatorToQuaternion` (.rotation (`SkinnedMeshComponent.GetBoneTransform` (`self.ReferenceMesh`) "lowerarm_l" "RTS_Component"))) (`KismetMathLibrary.Quat_Inversed` Quat_3))))

(fn `ComputeOffset4`
  (params (Quat_4 :type "Quat Structure"))
  (returns (Offset_4 :type "Quat Structure"))
  (return (* (`KismetMathLibrary.Conv_RotatorToQuaternion` (.rotation (`SkinnedMeshComponent.GetBoneTransform` (`self.ReferenceMesh`) "spine_03" "RTS_Component"))) (`KismetMathLibrary.Quat_Inversed` (`KismetMathLibrary.Conv_RotatorToQuaternion` (`KismetMathLibrary.MakeRotator` (.roll (`KismetMathLibrary.Quat_Rotator` Quat_4)) (.yaw (`KismetMathLibrary.Quat_Rotator` Quat_4)) (.pitch (`KismetMathLibrary.Quat_Rotator` Quat_4))))))))

(fn `ComputeOffsets`
  (params (Quat_0 :type "Quat Structure") (Quat_1 :type "Quat Structure") (Quat_2 :type "Quat Structure") (Quat_3 :type "Quat Structure") (Quat_4 :type "Quat Structure"))
  (returns (Quat_0_Offset :type "Quat Structure") (Quat_1_Offset :type "Quat Structure") (Quat_2_Offset :type "Quat Structure") (Quat_3_Offset :type "Quat Structure") (Quat_4_Offset :type "Quat Structure"))
  (return (* (`KismetMathLibrary.Conv_RotatorToQuaternion` (.rotation (`SkinnedMeshComponent.GetBoneTransform` (`self.ReferenceMesh`) "upperarm_l" "RTS_Component"))) (`KismetMathLibrary.Quat_Inversed` Quat_1)) (* (`KismetMathLibrary.Conv_RotatorToQuaternion` (.rotation (`SkinnedMeshComponent.GetBoneTransform` (`self.ReferenceMesh`) "upperarm_r" "RTS_Component"))) (`KismetMathLibrary.Quat_Inversed` Quat_0)) (* (`KismetMathLibrary.Conv_RotatorToQuaternion` (.rotation (`SkinnedMeshComponent.GetBoneTransform` (`self.ReferenceMesh`) "lowerarm_l" "RTS_Component"))) (`KismetMathLibrary.Quat_Inversed` Quat_3)) (* (`KismetMathLibrary.Conv_RotatorToQuaternion` (.rotation (`SkinnedMeshComponent.GetBoneTransform` (`self.ReferenceMesh`) "lowerarm_r" "RTS_Component"))) (`KismetMathLibrary.Quat_Inversed` Quat_2)) (* (`KismetMathLibrary.Conv_RotatorToQuaternion` (.rotation (`SkinnedMeshComponent.GetBoneTransform` (`self.ReferenceMesh`) "spine_03" "RTS_Component"))) (`KismetMathLibrary.Quat_Inversed` Quat_4))))

(fn `MirrorQuatFB`
  (params (InQuat :type "Quat Structure"))
  (returns (OutQuat :type "Quat Structure"))
  (bind (_x _y _z _w) (`KismetMathLibrary.BreakQuat` InQuat))
  (return (`KismetMathLibrary.MakeQuat` (* _x -1.0) _y (* _z -1.0) _w)))

(fn `MirrorQuatLR`
  (params (InQuat :type "Quat Structure"))
  (returns (OutQuat :type "Quat Structure"))
  (bind (_x _y _z _w) (`KismetMathLibrary.BreakQuat` InQuat))
  (return (`KismetMathLibrary.MakeQuat` _x (* _y -1.0) (* _z -1.0) _w)))

(fn `UserConstructionScript`)